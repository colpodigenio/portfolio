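; Gameplay player controller that sets up each local player's score sheet and match menu, and publishes their name and picture.
; On BeginPlay, profile data from the game instance goes into GameplayPlayerState, directly with authority or through ServerSetPlayerName on clients.
; The MatchMenu input shows the menu with UI-only input, and EndMatch destroys the session.
; The construction script separately loads saved player info into its own PlayerInfo.
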(event Custom|EndMatch
  ;[1 1 1] End Match
  (bind _asbp_game_instance (Utilities|Casting|CastToBP_GameInstance (Game|GetGameInstance)))
  (Default|DestroySession _asbp_game_instance self))

(event Custom|ServerSetPlayerName
  (params (PlayerName :type Name) (PlayerPicture :type Texture%202D%20Object%20Reference))
  ;[1 1 1] Set players name on clients
  (bind _asgameplay_player_state (Utilities|Casting|CastToGameplayPlayerState (Variables|Default|GetPlayerState)))
  (Variables|/Script/portfolio_project.GameplayPlayerState|SetPlayerNickName _asgameplay_player_state PlayerName)
  (Variables|/Script/portfolio_project.GameplayPlayerState|SetPlayerPicture _asgameplay_player_state PlayerPicture))

(event EventBeginPlay
  (Input|SetInputModeGameOnly self)
  (Utilities|FlowControl|Sequence
    (:then_0
      (if (Pawn|IsLocalController)
        ;[1 1 1] Creates score sheet widget
        (bind _returnvalue (UserInterface|CreateWidget "/Game/UI/ScoreSheet.ScoreSheet_C" self))
        (bind _output_get (Variables|Default|SetScoreSheetWidget _returnvalue))
        (Utilities|IsValid _output_get
          (:Is%20Valid
            (Variables|/Game/UI/ScoreSheet.ScoreSheet_C|SetOwningPlayer _output_get self)
            (UserInterface|Viewport|AddtoViewport _output_get 0)))))
    (:then_1
      (Networking|SwitchHasAuthority
        (:Authority
          (if (Pawn|IsLocalController)
            ;[1 1 1] Set Players Name on listen server in Player State to show it in Score Sheet
            (bind _asgameplay_player_state (Utilities|Casting|CastToGameplayPlayerState (Variables|Default|GetPlayerState)))
            (bind _asbp_game_instance (Utilities|Casting|CastToBP_GameInstance (Game|GetGameInstance)))
            (Variables|/Script/portfolio_project.GameplayPlayerState|SetPlayerNickName _asgameplay_player_state (.playername (Variables|/Game/Blueprints/Global/BP_GameInstance.BP_GameInstance_C|GetPlayerInfo _asbp_game_instance)))
            (Variables|/Script/portfolio_project.GameplayPlayerState|SetPlayerPicture _asgameplay_player_state (.playerpicture (Variables|/Game/Blueprints/Global/BP_GameInstance.BP_GameInstance_C|GetPlayerInfo _asbp_game_instance)))))
        (:Remote
          (if (Pawn|IsLocalController)
            ;[1 1 1] Set players name on clients
            (bind _asbp_game_instance_2 (Utilities|Casting|CastToBP_GameInstance (Game|GetGameInstance)))
            (Development|PrintString (Utilities|String|ToString(Name) (.playername (Variables|/Game/Blueprints/Global/BP_GameInstance.BP_GameInstance_C|GetPlayerInfo _asbp_game_instance_2))))
            (CallFunction|ServerSetPlayerName (.playername (Variables|/Game/Blueprints/Global/BP_GameInstance.BP_GameInstance_C|GetPlayerInfo _asbp_game_instance_2)) (.playerpicture (Variables|/Game/Blueprints/Global/BP_GameInstance.BP_GameInstance_C|GetPlayerInfo _asbp_game_instance_2)))))))
    (:then_2
      ;[1 1 1] Create Match Menu
      (if (Pawn|IsLocalController)
        (bind _returnvalue_2 (UserInterface|CreateWidget "/Game/UI/MainMenu/MatchMenu.MatchMenu_C" self))
        (Variables|Default|SetMatchMenuInst _returnvalue_2)))))

(event EventTick
  (params (DeltaSeconds :type Float%20%28single-precision%29)))

(event Input|ActionEvents|InputActionMatchMenu
  (params (Key :type Key%20Structure))
  ;[1 1 1] Show Match Menu
  (:Pressed
    (UserInterface|Viewport|AddtoViewport (Variables|Default|GetMatchMenuInst) 0)
    (Input|SetInputModeUIOnly self 0 "DoNotLock")
    (Variables|Default|SetbShowMouseCursor true)))

(fn ConstructionScript
  (bind _returnvalue (SaveGame|LoadGamefromSlot "PlayerSettingsSaveGame"))
  (bind _asplayer_save_game (Utilities|Casting|CastToPlayerSaveGame _returnvalue))
  (Variables|Default|SetPlayerInfo (Variables|/Script/portfolio_project.PlayerSaveGame|GetSavePlayerInfo _asplayer_save_game)))