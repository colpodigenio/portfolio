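; BP_LaunchPad is a launch pad that throws an overlapping FPSCharacter and plays a launch sound at the pad.
; On overlap it calls LaunchCharacter with LaunchDestination used directly as the velocity, overriding existing XY and Z movement.
; The construction script creates a dynamic material on the Cube and feeds IsLaunchPadVertical into its LaunchPadType scalar parameter, which affects only the material, not the launch.
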(event Collision|EventActorBeginOverlap
  (params (OtherActor :type Actor%20Object%20Reference))
  (bind _asfpscharacter (Utilities|Casting|CastToFPSCharacter OtherActor))
  (Character|LaunchCharacter _asfpscharacter (Variables|Default|GetLaunchDestination) true true)
  (Audio|PlaySoundatLocation (Variables|Default|GetLaunchSound) (Transformation|GetActorLocation) "0, 0, 0" 1.0 1.0 0.0 0 0 0))

(fn ConstructionScript
  (bind _returnvalue (Rendering|Material|CreateDynamicMaterialInstance (Variables|Default|GetCube) 0 "/Game/Assets/Materials/LaunchPadMaterial.LaunchPadMaterial" "LaunchPadType" :!class /Script/Engine.PrimitiveComponent))
  (Rendering|Material|SetScalarParameterValue _returnvalue "LaunchPadType" (Variables|Default|GetIsLaunchPadVertical) :!class /Script/Engine.MaterialInstanceDynamic))