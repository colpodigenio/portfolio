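; Behavior tree service that picks the nearest living FPSCharacter an AI pawn perceives by sight and sets it as the attack target.
; Each tick it scans known sight-perceived actors, skipping itself and dead characters, and keeps the closest by distance.
; It writes the result to a blackboard key, then resets the distance threshold but not the stored target, so the previous pick persists when none qualifies.
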(event EventReceiveTickAI
  (params (OwnerController :type AI%20Controller%20Object%20Reference) (ControlledPawn :type Pawn%20Object%20Reference) (DeltaSeconds :type Float%20%28single-precision%29))
  (for _array_element (Class|AIPerceptionComponent|GetKnownPerceivedActors (Actor|GetComponentbyClass ControlledPawn "/Script/AIModule.AIPerceptionComponent") "/Script/AIModule.AISense_Sight")
    (bind _asfpscharacter (Utilities|Casting|CastToFPSCharacter _array_element))
    (if (Math|Boolean|ANDBoolean (not (Variables|/Script/portfolio_project.FPSCharacter|GetbIsDead _asfpscharacter)) (!= _array_element ControlledPawn) (< (Math|Vector|VectorLength (- (Transformation|GetActorLocation ControlledPawn) (Transformation|GetActorLocation _array_element))) (Variables|Default|GetDistanceToTarget)))
      (Variables|Default|SetTargetToAttack _asfpscharacter)
      (Variables|Default|SetDistanceToTarget (Math|Vector|VectorLength (- (Transformation|GetActorLocation ControlledPawn) (Transformation|GetActorLocation _array_element))))))
  (Class|BTFunctionLibrary|SetBlackboardValueasObject (Variables|Default|GetBBKeyTargetToAttack) (Variables|Default|GetTargetToAttack))
  (Variables|Default|SetDistanceToTarget 1e+06))