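; Behavior tree service that copies an AI-controlled FPS character's own combat state into its blackboard.
; On each AI tick it casts the pawn to FPSCharacter, then writes health, assault rifle reserve ammo and magazine ammo to Self-prefixed keys named by literals.
; It also calls ToggleActive on the HealthComponent every tick before reading health, flipping that component's active state each time.
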(event EventReceiveTickAI
  (params (OwnerController :type AI%20Controller%20Object%20Reference) (ControlledPawn :type Pawn%20Object%20Reference) (DeltaSeconds :type Float%20%28single-precision%29))
  (bind _returnvalue (AI|GetBlackboard ControlledPawn))
  (bind _asfpscharacter (Utilities|Casting|CastToFPSCharacter ControlledPawn))
  (Components|Activation|ToggleActive (Variables|/Script/portfolio_project.FPSCharacter|GetHealthComponent _asfpscharacter))
  (AI|Components|Blackboard|SetValueasFloat _returnvalue (Utilities|Name|MakeLiteralName "SelfHealth") (Variables|/Script/portfolio_project.HealthComponent|GetHealth (Variables|/Script/portfolio_project.FPSCharacter|GetHealthComponent _asfpscharacter)))
  (Class|BlackboardComponent|SetValueasInt _returnvalue (Utilities|Name|MakeLiteralName "SelfAssaultRifleAmmo") (Variables|/Script/portfolio_project.FPSCharacter|GetAssaultRifleAmmoAmount _asfpscharacter))
  (Class|BlackboardComponent|SetValueasInt _returnvalue (Utilities|Name|MakeLiteralName "SelfAssaultRifleAmmoInMagazine") (Variables|/Script/portfolio_project.FPSCharacter|GetAssaultRifleAmmoInMagazine _asfpscharacter)))