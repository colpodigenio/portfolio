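; Behavior Tree decorator that passes when the AI pawn is within attack distance of its target.
; It reads the target actor from a Blackboard key and compares the straight-line distance between the pawn and target locations to a distance threshold, inclusive.
; The condition fails when the target is not valid.
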(fn PerformConditionCheckAI
  (params (OwnerController :type AI%20Controller%20Object%20Reference) (ControlledPawn :type Pawn%20Object%20Reference))
  (bind _bbkeytargettoattack (Variables|Default|GetBBKeyTargetToAttack))
  (bind _returnvalue (AI|BehaviorTree|GetBlackboardValueasActor _bbkeytargettoattack))
  (Utilities|IsValid _returnvalue
    (:Is%20Valid
      (return (<= (Math|Vector|VectorLength (- (Transformation|GetActorLocation ControlledPawn) (Transformation|GetActorLocation _returnvalue))) (Variables|Default|GetDistanceToTargetToAttack))))
    (:Is%20Not%20Valid
      (return false))))