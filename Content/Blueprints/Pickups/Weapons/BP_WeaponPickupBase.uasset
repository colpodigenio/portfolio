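; Base weapon pickup that grants an assault rifle, shotgun or rocket launcher, selected by WeaponType, which also sets its preview mesh at construction.
; On supply, it reads the overlapping character from its owning PickupRespawn.
; An owned weapon gains NumberOfMagazines of ammo capped at the maximum; a missing one is spawned and assigned with a full magazine.
; The pickup then destroys itself.
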(event EventOnSupplyPickup
  (bind _aspickup_respawn (Utilities|Casting|CastToPickupRespawn (Components|GetOwner)))
  (switch Utilities|FlowControl|Switch|SwitchonEWeaponType (Variables|Default|GetWeaponType)
    (:AssaultRifle
      ;[1 1 1] Add Assault rifle
      (Utilities|IsValid (Variables|/Script/portfolio_project.FPSCharacter|GetAssaultRifle (Variables|/Script/portfolio_project.PickupRespawn|GetOverlappedCharacter _aspickup_respawn))
        (:Is%20Valid
          (if (> (+ (* (Variables|Default|GetNumberOfMagazines) (Variables|/Script/portfolio_project.FPSCharacter|GetAssaultRifleMagazineCapacity (Variables|/Script/portfolio_project.PickupRespawn|GetOverlappedCharacter _aspickup_respawn))) (Variables|/Script/portfolio_project.FPSCharacter|GetAssaultRifleAmmoAmount (Variables|/Script/portfolio_project.PickupRespawn|GetOverlappedCharacter _aspickup_respawn))) (Variables|/Script/portfolio_project.FPSCharacter|GetMaxAssaultRifleAmmoAmount (Variables|/Script/portfolio_project.PickupRespawn|GetOverlappedCharacter _aspickup_respawn)))
            (Variables|/Script/portfolio_project.FPSCharacter|SetAssaultRifleAmmoAmount (Variables|/Script/portfolio_project.PickupRespawn|GetOverlappedCharacter _aspickup_respawn) (Variables|/Script/portfolio_project.FPSCharacter|GetMaxAssaultRifleAmmoAmount (Variables|/Script/portfolio_project.PickupRespawn|GetOverlappedCharacter _aspickup_respawn)))
            (else
              (Variables|/Script/portfolio_project.FPSCharacter|SetAssaultRifleAmmoAmount (Variables|/Script/portfolio_project.PickupRespawn|GetOverlappedCharacter _aspickup_respawn) (+ (* (Variables|Default|GetNumberOfMagazines) (Variables|/Script/portfolio_project.FPSCharacter|GetAssaultRifleMagazineCapacity (Variables|/Script/portfolio_project.PickupRespawn|GetOverlappedCharacter _aspickup_respawn))) (Variables|/Script/portfolio_project.FPSCharacter|GetAssaultRifleAmmoAmount (Variables|/Script/portfolio_project.PickupRespawn|GetOverlappedCharacter _aspickup_respawn)))))))
        (:Is%20Not%20Valid
          (bind _returnvalue (Game|SpawnActorfromClass "/Game/Blueprints/Weapons/BP_AssaultRifle.BP_AssaultRifle_C" (Math|Transform|MakeTransform "0, 0, 0") "AlwaysSpawn" 0 0))
          (Variables|/Script/portfolio_project.FPSCharacter|SetAssaultRifle (Variables|/Script/portfolio_project.PickupRespawn|GetOverlappedCharacter _aspickup_respawn) _returnvalue)
          (Variables|/Script/portfolio_project.FPSCharacter|SetAssaultRifleAmmoAmount (Variables|/Script/portfolio_project.PickupRespawn|GetOverlappedCharacter _aspickup_respawn) (+ (Variables|/Script/portfolio_project.FPSCharacter|GetAssaultRifleMagazineCapacity (Variables|/Script/portfolio_project.PickupRespawn|GetOverlappedCharacter _aspickup_respawn)) (Variables|/Script/portfolio_project.FPSCharacter|GetAssaultRifleAmmoAmount (Variables|/Script/portfolio_project.PickupRespawn|GetOverlappedCharacter _aspickup_respawn))))
          (Variables|/Script/portfolio_project.FPSCharacter|SetAssaultRifleAmmoInMagazine (Variables|/Script/portfolio_project.PickupRespawn|GetOverlappedCharacter _aspickup_respawn) (Variables|/Script/portfolio_project.FPSCharacter|GetAssaultRifleMagazineCapacity (Variables|/Script/portfolio_project.PickupRespawn|GetOverlappedCharacter _aspickup_respawn))))))
    (:Shotgun
      ;[1 1 1] Add Shotgun ammo
      (Utilities|IsValid (Variables|/Script/portfolio_project.FPSCharacter|GetShotgun (Variables|/Script/portfolio_project.PickupRespawn|GetOverlappedCharacter _aspickup_respawn))
        (:Is%20Valid
          (if (> (+ (* (Variables|Default|GetNumberOfMagazines) (Variables|/Script/portfolio_project.FPSCharacter|GetShotgunMagazineCapacity (Variables|/Script/portfolio_project.PickupRespawn|GetOverlappedCharacter _aspickup_respawn))) (Variables|/Script/portfolio_project.FPSCharacter|GetShotgunAmmoAmount (Variables|/Script/portfolio_project.PickupRespawn|GetOverlappedCharacter _aspickup_respawn))) (Variables|/Script/portfolio_project.FPSCharacter|GetMaxShotgunAmmoAmount (Variables|/Script/portfolio_project.PickupRespawn|GetOverlappedCharacter _aspickup_respawn)))
            (Variables|/Script/portfolio_project.FPSCharacter|SetShotgunAmmoAmount (Variables|/Script/portfolio_project.PickupRespawn|GetOverlappedCharacter _aspickup_respawn) (Variables|/Script/portfolio_project.FPSCharacter|GetMaxShotgunAmmoAmount (Variables|/Script/portfolio_project.PickupRespawn|GetOverlappedCharacter _aspickup_respawn)))
            (else
              (Variables|/Script/portfolio_project.FPSCharacter|SetShotgunAmmoAmount (Variables|/Script/portfolio_project.PickupRespawn|GetOverlappedCharacter _aspickup_respawn) (+ (* (Variables|Default|GetNumberOfMagazines) (Variables|/Script/portfolio_project.FPSCharacter|GetShotgunMagazineCapacity (Variables|/Script/portfolio_project.PickupRespawn|GetOverlappedCharacter _aspickup_respawn))) (Variables|/Script/portfolio_project.FPSCharacter|GetShotgunAmmoAmount (Variables|/Script/portfolio_project.PickupRespawn|GetOverlappedCharacter _aspickup_respawn)))))))
        (:Is%20Not%20Valid
          (bind _returnvalue_2 (Game|SpawnActorfromClass "/Game/Blueprints/Weapons/BP_ShotGun.BP_Shotgun_C" (Math|Transform|MakeTransform "0, 0, 0") "AlwaysSpawn" 0 0))
          (Variables|/Script/portfolio_project.FPSCharacter|SetShotgun (Variables|/Script/portfolio_project.PickupRespawn|GetOverlappedCharacter _aspickup_respawn) _returnvalue_2)
          (Variables|/Script/portfolio_project.FPSCharacter|SetShotgunAmmoAmount (Variables|/Script/portfolio_project.PickupRespawn|GetOverlappedCharacter _aspickup_respawn) (+ (Variables|/Script/portfolio_project.FPSCharacter|GetShotgunMagazineCapacity (Variables|/Script/portfolio_project.PickupRespawn|GetOverlappedCharacter _aspickup_respawn)) (Variables|/Script/portfolio_project.FPSCharacter|GetShotgunAmmoAmount (Variables|/Script/portfolio_project.PickupRespawn|GetOverlappedCharacter _aspickup_respawn))))
          (Variables|/Script/portfolio_project.FPSCharacter|SetShotgunAmmoInMagazine (Variables|/Script/portfolio_project.PickupRespawn|GetOverlappedCharacter _aspickup_respawn) (Variables|/Script/portfolio_project.FPSCharacter|GetShotgunMagazineCapacity (Variables|/Script/portfolio_project.PickupRespawn|GetOverlappedCharacter _aspickup_respawn))))))
    (:RocketLauncher
      ;[1 1 1] Add Rocket launcher ammo
      (Utilities|IsValid (Variables|/Script/portfolio_project.FPSCharacter|GetRocketLauncher (Variables|/Script/portfolio_project.PickupRespawn|GetOverlappedCharacter _aspickup_respawn))
        (:Is%20Valid
          (if (> (+ (* (Variables|Default|GetNumberOfMagazines) (Variables|/Script/portfolio_project.FPSCharacter|GetRocketLauncherMagazineCapacity (Variables|/Script/portfolio_project.PickupRespawn|GetOverlappedCharacter _aspickup_respawn))) (Variables|/Script/portfolio_project.FPSCharacter|GetRocketLauncherAmmoAmount (Variables|/Script/portfolio_project.PickupRespawn|GetOverlappedCharacter _aspickup_respawn))) (Variables|/Script/portfolio_project.FPSCharacter|GetMaxRocketLauncherAmmoAmount (Variables|/Script/portfolio_project.PickupRespawn|GetOverlappedCharacter _aspickup_respawn)))
            (Variables|/Script/portfolio_project.FPSCharacter|SetRocketLauncherAmmoAmount (Variables|/Script/portfolio_project.PickupRespawn|GetOverlappedCharacter _aspickup_respawn) (Variables|/Script/portfolio_project.FPSCharacter|GetMaxRocketLauncherAmmoAmount (Variables|/Script/portfolio_project.PickupRespawn|GetOverlappedCharacter _aspickup_respawn)))
            (else
              (Variables|/Script/portfolio_project.FPSCharacter|SetRocketLauncherAmmoAmount (Variables|/Script/portfolio_project.PickupRespawn|GetOverlappedCharacter _aspickup_respawn) (+ (* (Variables|Default|GetNumberOfMagazines) (Variables|/Script/portfolio_project.FPSCharacter|GetRocketLauncherMagazineCapacity (Variables|/Script/portfolio_project.PickupRespawn|GetOverlappedCharacter _aspickup_respawn))) (Variables|/Script/portfolio_project.FPSCharacter|GetRocketLauncherAmmoAmount (Variables|/Script/portfolio_project.PickupRespawn|GetOverlappedCharacter _aspickup_respawn)))))))
        (:Is%20Not%20Valid
          (bind _returnvalue_3 (Game|SpawnActorfromClass "/Game/Blueprints/Weapons/BP_RocketLauncher.BP_RocketLauncher_C" (Math|Transform|MakeTransform "0, 0, 0") "AlwaysSpawn" 0 0))
          (Variables|/Script/portfolio_project.FPSCharacter|SetRocketLauncher (Variables|/Script/portfolio_project.PickupRespawn|GetOverlappedCharacter _aspickup_respawn) _returnvalue_3)
          (Variables|/Script/portfolio_project.FPSCharacter|SetRocketLauncherAmmoAmount (Variables|/Script/portfolio_project.PickupRespawn|GetOverlappedCharacter _aspickup_respawn) (+ (Variables|/Script/portfolio_project.FPSCharacter|GetRocketLauncherMagazineCapacity (Variables|/Script/portfolio_project.PickupRespawn|GetOverlappedCharacter _aspickup_respawn)) (Variables|/Script/portfolio_project.FPSCharacter|GetRocketLauncherAmmoAmount (Variables|/Script/portfolio_project.PickupRespawn|GetOverlappedCharacter _aspickup_respawn))))
          (Variables|/Script/portfolio_project.FPSCharacter|SetRocketLauncherAmmoInMagazine (Variables|/Script/portfolio_project.PickupRespawn|GetOverlappedCharacter _aspickup_respawn) (Variables|/Script/portfolio_project.FPSCharacter|GetRocketLauncherMagazineCapacity (Variables|/Script/portfolio_project.PickupRespawn|GetOverlappedCharacter _aspickup_respawn)))))))
  (Actor|DestroyActor))

(fn ConstructionScript
  (switch Utilities|FlowControl|Switch|SwitchonEWeaponType (Variables|Default|GetWeaponType)
    (:None
      (Class|SkinnedMeshComponent|SetSkeletalMesh (Variables|Default|GetPickupWeapon) 0 false))
    (:AssaultRifle
      (Class|SkinnedMeshComponent|SetSkeletalMesh (Variables|Default|GetPickupWeapon) "/Game/Assets/Weapons/SK_Rifle.SK_Rifle" false))
    (:Shotgun
      (Class|SkinnedMeshComponent|SetSkeletalMesh (Variables|Default|GetPickupWeapon) "/Game/Assets/FPWeapon/Mesh/SK_FPGun.SK_FPGun" false))
    (:RocketLauncher
      (Class|SkinnedMeshComponent|SetSkeletalMesh (Variables|Default|GetPickupWeapon) "/Game/Assets/Weapons/Launcher.Launcher" false))))