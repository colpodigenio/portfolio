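; Base supply pickup that gives ammo, grenades, mines, health or armor to a character, chosen by SupplyType.
; Its construction script sets the matching mesh for that type.
; OnSupplyPickup reads OverlappedCharacter from its PickupRespawn owner, adds the amount capped at maximum, then destroys itself.
; Only health and armor writes are authority-gated, and mine overflow sets the count to zero instead of the maximum.
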(event EventOnSupplyPickup
  (switch Utilities|FlowControl|Switch|SwitchonESupplyType (Variables|Default|GetSupplyType)
    (:AssaultRifleAmmo
      ;[1 1 1] Add Assault rifle ammo
      (bind _aspickup_respawn (Utilities|Casting|CastToPickupRespawn (Components|GetOwner)))
      (if (> (+ (* (Variables|Default|GetNumberOfMagazines) (Variables|/Script/portfolio_project.FPSCharacter|GetAssaultRifleMagazineCapacity (Variables|/Script/portfolio_project.PickupRespawn|GetOverlappedCharacter _aspickup_respawn))) (Variables|/Script/portfolio_project.FPSCharacter|GetAssaultRifleAmmoAmount (Variables|/Script/portfolio_project.PickupRespawn|GetOverlappedCharacter _aspickup_respawn))) (Variables|/Script/portfolio_project.FPSCharacter|GetMaxAssaultRifleAmmoAmount (Variables|/Script/portfolio_project.PickupRespawn|GetOverlappedCharacter _aspickup_respawn)))
        (Variables|/Script/portfolio_project.FPSCharacter|SetAssaultRifleAmmoAmount (Variables|/Script/portfolio_project.PickupRespawn|GetOverlappedCharacter _aspickup_respawn) (Variables|/Script/portfolio_project.FPSCharacter|GetMaxAssaultRifleAmmoAmount (Variables|/Script/portfolio_project.PickupRespawn|GetOverlappedCharacter _aspickup_respawn)))
        (else
          (Variables|/Script/portfolio_project.FPSCharacter|SetAssaultRifleAmmoAmount (Variables|/Script/portfolio_project.PickupRespawn|GetOverlappedCharacter _aspickup_respawn) (+ (* (Variables|Default|GetNumberOfMagazines) (Variables|/Script/portfolio_project.FPSCharacter|GetAssaultRifleMagazineCapacity (Variables|/Script/portfolio_project.PickupRespawn|GetOverlappedCharacter _aspickup_respawn))) (Variables|/Script/portfolio_project.FPSCharacter|GetAssaultRifleAmmoAmount (Variables|/Script/portfolio_project.PickupRespawn|GetOverlappedCharacter _aspickup_respawn))))))
      (Actor|DestroyActor :!label _label))
    (:ShotgunAmmo
      ;[1 1 1] Add Shotgun ammo
      (bind _aspickup_respawn_2 (Utilities|Casting|CastToPickupRespawn (Components|GetOwner)))
      (if (> (+ (* (Variables|Default|GetNumberOfMagazines) (Variables|/Script/portfolio_project.FPSCharacter|GetShotgunMagazineCapacity (Variables|/Script/portfolio_project.PickupRespawn|GetOverlappedCharacter _aspickup_respawn_2))) (Variables|/Script/portfolio_project.FPSCharacter|GetShotgunAmmoAmount (Variables|/Script/portfolio_project.PickupRespawn|GetOverlappedCharacter _aspickup_respawn_2))) (Variables|/Script/portfolio_project.FPSCharacter|GetMaxShotgunAmmoAmount (Variables|/Script/portfolio_project.PickupRespawn|GetOverlappedCharacter _aspickup_respawn_2)))
        (Variables|/Script/portfolio_project.FPSCharacter|SetShotgunAmmoAmount (Variables|/Script/portfolio_project.PickupRespawn|GetOverlappedCharacter _aspickup_respawn_2) (Variables|/Script/portfolio_project.FPSCharacter|GetMaxShotgunAmmoAmount (Variables|/Script/portfolio_project.PickupRespawn|GetOverlappedCharacter _aspickup_respawn_2)))
        (goto _label)
        (else
          (Variables|/Script/portfolio_project.FPSCharacter|SetShotgunAmmoAmount (Variables|/Script/portfolio_project.PickupRespawn|GetOverlappedCharacter _aspickup_respawn_2) (+ (* (Variables|Default|GetNumberOfMagazines) (Variables|/Script/portfolio_project.FPSCharacter|GetShotgunMagazineCapacity (Variables|/Script/portfolio_project.PickupRespawn|GetOverlappedCharacter _aspickup_respawn_2))) (Variables|/Script/portfolio_project.FPSCharacter|GetShotgunAmmoAmount (Variables|/Script/portfolio_project.PickupRespawn|GetOverlappedCharacter _aspickup_respawn_2))))
          (goto _label))))
    (:RocketLauncherAmmo
      ;[1 1 1] Add Rocket launcher ammo
      (bind _aspickup_respawn_3 (Utilities|Casting|CastToPickupRespawn (Components|GetOwner)))
      (if (> (+ (* (Variables|Default|GetNumberOfMagazines) (Variables|/Script/portfolio_project.FPSCharacter|GetRocketLauncherMagazineCapacity (Variables|/Script/portfolio_project.PickupRespawn|GetOverlappedCharacter _aspickup_respawn_3))) (Variables|/Script/portfolio_project.FPSCharacter|GetRocketLauncherAmmoAmount (Variables|/Script/portfolio_project.PickupRespawn|GetOverlappedCharacter _aspickup_respawn_3))) (Variables|/Script/portfolio_project.FPSCharacter|GetMaxRocketLauncherAmmoAmount (Variables|/Script/portfolio_project.PickupRespawn|GetOverlappedCharacter _aspickup_respawn_3)))
        (Variables|/Script/portfolio_project.FPSCharacter|SetRocketLauncherAmmoAmount (Variables|/Script/portfolio_project.PickupRespawn|GetOverlappedCharacter _aspickup_respawn_3) (Variables|/Script/portfolio_project.FPSCharacter|GetMaxRocketLauncherAmmoAmount (Variables|/Script/portfolio_project.PickupRespawn|GetOverlappedCharacter _aspickup_respawn_3)))
        (goto _label)
        (else
          (Variables|/Script/portfolio_project.FPSCharacter|SetRocketLauncherAmmoAmount (Variables|/Script/portfolio_project.PickupRespawn|GetOverlappedCharacter _aspickup_respawn_3) (+ (* (Variables|Default|GetNumberOfMagazines) (Variables|/Script/portfolio_project.FPSCharacter|GetRocketLauncherMagazineCapacity (Variables|/Script/portfolio_project.PickupRespawn|GetOverlappedCharacter _aspickup_respawn_3))) (Variables|/Script/portfolio_project.FPSCharacter|GetRocketLauncherAmmoAmount (Variables|/Script/portfolio_project.PickupRespawn|GetOverlappedCharacter _aspickup_respawn_3))))
          (goto _label))))
    (:Grenade
      ;[1 1 1] Add grenades
      (bind _aspickup_respawn_4 (Utilities|Casting|CastToPickupRespawn (Components|GetOwner)))
      (if (> (+ (Variables|/Script/portfolio_project.FPSCharacter|GetGrenadesAmount (Variables|/Script/portfolio_project.PickupRespawn|GetOverlappedCharacter _aspickup_respawn_4)) 3) (Variables|/Script/portfolio_project.FPSCharacter|GetMaxGrenadesAmount (Variables|/Script/portfolio_project.PickupRespawn|GetOverlappedCharacter _aspickup_respawn_4)))
        (Variables|/Script/portfolio_project.FPSCharacter|SetGrenadesAmount (Variables|/Script/portfolio_project.PickupRespawn|GetOverlappedCharacter _aspickup_respawn_4) (Variables|/Script/portfolio_project.FPSCharacter|GetMaxGrenadesAmount (Variables|/Script/portfolio_project.PickupRespawn|GetOverlappedCharacter _aspickup_respawn_4)))
        (goto _label)
        (else
          (Variables|/Script/portfolio_project.FPSCharacter|SetGrenadesAmount (Variables|/Script/portfolio_project.PickupRespawn|GetOverlappedCharacter _aspickup_respawn_4) (+ (Variables|/Script/portfolio_project.FPSCharacter|GetGrenadesAmount (Variables|/Script/portfolio_project.PickupRespawn|GetOverlappedCharacter _aspickup_respawn_4)) 3))
          (goto _label))))
    (:Mine
      ;[1 1 1] Add remote bombs
      (bind _aspickup_respawn_5 (Utilities|Casting|CastToPickupRespawn (Components|GetOwner)))
      (if (> (+ (Variables|/Script/portfolio_project.FPSCharacter|GetMinesAmount (Variables|/Script/portfolio_project.PickupRespawn|GetOverlappedCharacter _aspickup_respawn_5)) 2) (Variables|/Script/portfolio_project.FPSCharacter|GetMaxMinesAmount (Variables|/Script/portfolio_project.PickupRespawn|GetOverlappedCharacter _aspickup_respawn_5)))
        (Variables|/Script/portfolio_project.FPSCharacter|SetMinesAmount (Variables|/Script/portfolio_project.PickupRespawn|GetOverlappedCharacter _aspickup_respawn_5) 0)
        (goto _label)
        (else
          (Variables|/Script/portfolio_project.FPSCharacter|SetMinesAmount (Variables|/Script/portfolio_project.PickupRespawn|GetOverlappedCharacter _aspickup_respawn_5) (+ (Variables|/Script/portfolio_project.FPSCharacter|GetMinesAmount (Variables|/Script/portfolio_project.PickupRespawn|GetOverlappedCharacter _aspickup_respawn_5)) 2))
          (goto _label))))
    (:Meds
      ;[1 1 1] Add health
      (bind _aspickup_respawn_6 (Utilities|Casting|CastToPickupRespawn (Components|GetOwner)))
      (if (and (<= (Variables|/Script/portfolio_project.HealthComponent|GetHealth (Variables|/Script/portfolio_project.FPSCharacter|GetHealthComponent (Variables|/Script/portfolio_project.PickupRespawn|GetOverlappedCharacter _aspickup_respawn_6))) (Class|HealthComponent|GetMaxHealth (Variables|/Script/portfolio_project.FPSCharacter|GetHealthComponent (Variables|/Script/portfolio_project.PickupRespawn|GetOverlappedCharacter _aspickup_respawn_6)))) (> (+ (Variables|/Script/portfolio_project.HealthComponent|GetHealth (Variables|/Script/portfolio_project.FPSCharacter|GetHealthComponent (Variables|/Script/portfolio_project.PickupRespawn|GetOverlappedCharacter _aspickup_respawn_6))) (Variables|Default|GetDeltaHealth)) (Class|HealthComponent|GetMaxHealth (Variables|/Script/portfolio_project.FPSCharacter|GetHealthComponent (Variables|/Script/portfolio_project.PickupRespawn|GetOverlappedCharacter _aspickup_respawn_6)))))
        (Networking|SwitchHasAuthority
          (:Authority
            (Variables|/Script/portfolio_project.HealthComponent|SetHealth (Variables|/Script/portfolio_project.FPSCharacter|GetHealthComponent (Variables|/Script/portfolio_project.PickupRespawn|GetOverlappedCharacter _aspickup_respawn_6)) (Class|HealthComponent|GetMaxHealth (Variables|/Script/portfolio_project.FPSCharacter|GetHealthComponent (Variables|/Script/portfolio_project.PickupRespawn|GetOverlappedCharacter _aspickup_respawn_6))))
            (goto _label)))
        (elif (<= (Variables|/Script/portfolio_project.HealthComponent|GetHealth (Variables|/Script/portfolio_project.FPSCharacter|GetHealthComponent (Variables|/Script/portfolio_project.PickupRespawn|GetOverlappedCharacter _aspickup_respawn_6))) (Class|HealthComponent|GetMaxHealth (Variables|/Script/portfolio_project.FPSCharacter|GetHealthComponent (Variables|/Script/portfolio_project.PickupRespawn|GetOverlappedCharacter _aspickup_respawn_6))))
          (Networking|SwitchHasAuthority
            (:Authority
              (Variables|/Script/portfolio_project.HealthComponent|SetHealth (Variables|/Script/portfolio_project.FPSCharacter|GetHealthComponent (Variables|/Script/portfolio_project.PickupRespawn|GetOverlappedCharacter _aspickup_respawn_6)) (+ (Variables|/Script/portfolio_project.HealthComponent|GetHealth (Variables|/Script/portfolio_project.FPSCharacter|GetHealthComponent (Variables|/Script/portfolio_project.PickupRespawn|GetOverlappedCharacter _aspickup_respawn_6))) (Variables|Default|GetDeltaHealth)))
              (goto _label))))))
    (:Armor
      ;[1 1 1] Add armor
      (bind _aspickup_respawn_7 (Utilities|Casting|CastToPickupRespawn (Components|GetOwner)))
      (if (> (+ (Variables|/Script/portfolio_project.HealthComponent|GetArmor (Variables|/Script/portfolio_project.FPSCharacter|GetHealthComponent (Variables|/Script/portfolio_project.PickupRespawn|GetOverlappedCharacter _aspickup_respawn_7))) (Variables|Default|GetDeltaArmor)) (Class|HealthComponent|GetMaxArmor (Variables|/Script/portfolio_project.FPSCharacter|GetHealthComponent (Variables|/Script/portfolio_project.PickupRespawn|GetOverlappedCharacter _aspickup_respawn_7))))
        (Networking|SwitchHasAuthority
          (:Authority
            (Variables|/Script/portfolio_project.HealthComponent|SetArmor (Variables|/Script/portfolio_project.FPSCharacter|GetHealthComponent (Variables|/Script/portfolio_project.PickupRespawn|GetOverlappedCharacter _aspickup_respawn_7)) (Class|HealthComponent|GetMaxArmor (Variables|/Script/portfolio_project.FPSCharacter|GetHealthComponent (Variables|/Script/portfolio_project.PickupRespawn|GetOverlappedCharacter _aspickup_respawn_7))))
            (goto _label)))
        (else
          (Networking|SwitchHasAuthority
            (:Authority
              (Variables|/Script/portfolio_project.HealthComponent|SetArmor (Variables|/Script/portfolio_project.FPSCharacter|GetHealthComponent (Variables|/Script/portfolio_project.PickupRespawn|GetOverlappedCharacter _aspickup_respawn_7)) (+ (Variables|/Script/portfolio_project.HealthComponent|GetArmor (Variables|/Script/portfolio_project.FPSCharacter|GetHealthComponent (Variables|/Script/portfolio_project.PickupRespawn|GetOverlappedCharacter _aspickup_respawn_7))) (Variables|Default|GetDeltaArmor)))
              (goto _label))))))))

(fn ConstructionScript
  (switch Utilities|FlowControl|Switch|SwitchonESupplyType (Variables|Default|GetSupplyType)
    (:None
      (Components|StaticMesh|SetStaticMesh (Variables|Default|GetPickupSupply) 0))
    (:AssaultRifleAmmo
      (Components|StaticMesh|SetStaticMesh (Variables|Default|GetPickupSupply) "/Game/Assets/Pickups/SupplyAssaultRifle.SupplyAssaultRifle"))
    (:ShotgunAmmo
      (Components|StaticMesh|SetStaticMesh (Variables|Default|GetPickupSupply) "/Game/Assets/Pickups/SupplyShotgun.SupplyShotgun"))
    (:RocketLauncherAmmo
      (Components|StaticMesh|SetStaticMesh (Variables|Default|GetPickupSupply) "/Game/Assets/Pickups/SupplyRocketLauncher.SupplyRocketLauncher"))
    (:Grenade
      (Components|StaticMesh|SetStaticMesh (Variables|Default|GetPickupSupply) "/Game/Assets/Pickups/SupplyGrenades.SupplyGrenades"))
    (:Mine
      (Components|StaticMesh|SetStaticMesh (Variables|Default|GetPickupSupply) "/Game/Assets/Pickups/SupplyMines.SupplyMines"))
    (:Meds
      (Components|StaticMesh|SetStaticMesh (Variables|Default|GetPickupSupply) "/Game/Assets/Pickups/SupplyHealth.SupplyHealth"))
    (:Armor
      (Components|StaticMesh|SetStaticMesh (Variables|Default|GetPickupSupply) "/Game/Assets/Pickups/SupplyArmor.SupplyArmor"))))