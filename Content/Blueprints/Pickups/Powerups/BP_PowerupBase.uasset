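; BP_PowerupBase is a base powerup pickup offering Speed Boost, Damage Boost or Regeneration, chosen by PowerupType.
; The construction script sets the matching icon mesh.
; Activation sets user flags and multiplies walk speed for Speed Boost, while ticks add health up to double maximum for Regeneration.
; Expiry reverts speed or ends damage boost on the user's three weapons, then destroys the actor; Regeneration has no expiry branch.
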(event EventOnPoweruponTick
  (bind _powerupuser (Variables|Default|GetPowerupUser))
  (bind _healthcomponent (Variables|/Script/portfolio_project.FPSCharacter|GetHealthComponent _powerupuser))
  (bind _returnvalue (Class|HealthComponent|GetMaxHealth _healthcomponent))
  (bind _returnvalue_2 (* _returnvalue 2.0))
  (Utilities|IsValid (Variables|Default|GetPowerupUser)
    (:Is%20Valid
      (switch Utilities|FlowControl|Switch|SwitchonEPowerupType (Variables|Default|GetPowerupType)
        (:Regeneration
          (if (> (+ (Variables|Default|GetRegeneratingHealthOnTick) (Variables|/Script/portfolio_project.HealthComponent|GetHealth _healthcomponent)) _returnvalue_2)
            (Variables|/Script/portfolio_project.HealthComponent|SetHealth _healthcomponent _returnvalue_2)
            (else
              (Variables|/Script/portfolio_project.HealthComponent|SetHealth _healthcomponent (+ (Variables|Default|GetRegeneratingHealthOnTick) (Variables|/Script/portfolio_project.HealthComponent|GetHealth _healthcomponent))))))))))

(event EventOnPoweruponTimeActivated
  (bind _powerupuser (Variables|Default|GetPowerupUser))
  (Utilities|IsValid (Variables|Default|GetPowerupUser)
    (:Is%20Valid
      (switch Utilities|FlowControl|Switch|SwitchonEPowerupType (Variables|Default|GetPowerupType)
        (:SpeedBoost
          (Variables|/Script/portfolio_project.FPSCharacter|SetbIsSpeedBoosted _powerupuser true)
          (Variables|/Script/Engine.CharacterMovementComponent|SetMaxWalkSpeed (Variables|/Script/Engine.Character|GetCharacterMovement (Variables|Default|GetPowerupUser)) (* (Class|MovementComponent|GetMaxSpeed (Variables|/Script/Engine.Character|GetCharacterMovement (Variables|Default|GetPowerupUser))) 1.5)))
        (:DamageBoost
          (Variables|/Script/portfolio_project.FPSCharacter|SetbIsDamageBoosted _powerupuser true))))))

(event EventOnPoweruponTimeExpired
  (Utilities|IsValid (Variables|Default|GetPowerupUser)
    (:Is%20Valid
      (switch Utilities|FlowControl|Switch|SwitchonEPowerupType (Variables|Default|GetPowerupType)
        (:SpeedBoost
          (Variables|/Script/portfolio_project.FPSCharacter|SetbIsSpeedBoosted (Variables|Default|GetPowerupUser) false)
          (Variables|/Script/portfolio_project.FPSCharacter|SetbIsPowerupActive (Variables|Default|GetPowerupUser) false)
          (Variables|/Script/Engine.CharacterMovementComponent|SetMaxWalkSpeed (Variables|/Script/Engine.Character|GetCharacterMovement (Variables|Default|GetPowerupUser)) (/ (Class|MovementComponent|GetMaxSpeed (Variables|/Script/Engine.Character|GetCharacterMovement (Variables|Default|GetPowerupUser))) 1.5))
          (Variables|Default|SetPowerupUser 0)
          (Actor|DestroyActor))
        (:DamageBoost
          (CallFunction|DamageBoostEnd)
          (Variables|/Script/portfolio_project.FPSCharacter|SetbIsPowerupActive (Variables|Default|GetPowerupUser) false)
          (Variables|/Script/portfolio_project.FPSCharacter|SetbIsDamageBoosted (Variables|Default|GetPowerupUser) false)
          (Variables|Default|SetPowerupUser 0)
          (Actor|DestroyActor))))))

(fn ConstructionScript
  (bind _pickupsupply (Variables|Default|GetPickupSupply))
  (switch Utilities|FlowControl|Switch|SwitchonEPowerupType (Variables|Default|GetPowerupType)
    (:None
      (Components|StaticMesh|SetStaticMesh _pickupsupply 0))
    (:SpeedBoost
      (Components|StaticMesh|SetStaticMesh _pickupsupply "/Game/Assets/Pickups/SpeedIcon.SpeedIcon"))
    (:DamageBoost
      (Components|StaticMesh|SetStaticMesh _pickupsupply "/Game/Assets/Pickups/DamageBoostIcon.DamageBoostIcon"))
    (:Regeneration
      (Components|StaticMesh|SetStaticMesh _pickupsupply "/Game/Assets/Pickups/HealthIcon.HealthIcon"))))

(fn DamageBoostEnd
  (bind _powerupuser (Variables|Default|GetPowerupUser))
  (bind _assaultrifle (Variables|/Script/portfolio_project.FPSCharacter|GetAssaultRifle _powerupuser))
  (bind _rocketlauncher (Variables|/Script/portfolio_project.FPSCharacter|GetRocketLauncher _powerupuser))
  (bind _shotgun (Variables|/Script/portfolio_project.FPSCharacter|GetShotgun _powerupuser))
  (Utilities|IsValid _assaultrifle
    (:Is%20Valid
      (Utilities|FlowControl|Sequence
        (:then_0
          (Class|Weapon|DamageBoostEnd _assaultrifle))
        (:then_1
          (Utilities|IsValid _shotgun :!label _label
            (:Is%20Valid
              (Utilities|FlowControl|Sequence
                (:then_0
                  (Class|Weapon|DamageBoostEnd _shotgun))
                (:then_1
                  (Utilities|IsValid _rocketlauncher :!label _label_2
                    (:Is%20Valid
                      (Class|Weapon|DamageBoostEnd _rocketlauncher))))))
            (:Is%20Not%20Valid
              (goto _label_2))))))
    (:Is%20Not%20Valid
      (goto _label))))